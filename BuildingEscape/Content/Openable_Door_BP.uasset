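; Openable door actor that swings open and closed when it receives open or close door events.
; It caches its initial rotation on BeginPlay, then a DoorSwing timeline adds a yaw offset to that rotation on each update.
; An event track on the timeline plays a lock sound at the door's location, and closing reverses the same timeline.
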(event OnClose(FDoorEvent)
  ;[1 1 1] Door Movement
  (bind _open_door (Timeline|Door%20Swing Reverse)
    (:Update
      (Transformation|SetActorRotation (Math|Rotator|CombineRotators (Variables|Default|GetInitial%20Rotation) (Math|Rotator|MakeRotator 0.0 0.0 _open_door))))
    (:Audio
      ;[1 1 1] Sound
      (Audio|PlaySoundatLocation "/Game/Audio/door-lock.door-lock" (Transformation|GetActorLocation)))))

(event OnOpen(FDoorEvent)
  ;[1 1 1] Door Movement
  (bind _open_door (Timeline|Door%20Swing Play)
    (:Update
      (Transformation|SetActorRotation (Math|Rotator|CombineRotators (Variables|Default|GetInitial%20Rotation) (Math|Rotator|MakeRotator 0.0 0.0 _open_door))))
    (:Audio
      ;[1 1 1] Sound
      (Audio|PlaySoundatLocation "/Game/Audio/door-lock.door-lock" (Transformation|GetActorLocation)))))

(event EventBeginPlay
  ;[1 1 1] Initial Door Rotation
  (Variables|Default|SetInitial%20Rotation (Transformation|GetActorRotation)))

(fn ConstructionScript)