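; Movable Blueprint that slides a target actor by a set offset when a trigger actor fires its mover event.
; BeginPlay converts the offset into a world destination and binds TriggerEvent to the trigger's Mover_BP dispatcher.
; Once triggered, Tick moves the target at constant DeltaMove velocity until it nears the destination.
; On arrival it stops, but unbinds the empty CustomEvennt rather than TriggerEvent, which stays bound.
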(event Custom|CustomEvennt)

(event Custom|TriggerEvent
  (Variables|Default|SetAllowMovement true))

(event EventBeginPlay
  (Utilities|FlowControl|Sequence
    (:then_0
      (Variables|Default|SetPositionOffset (+ (Transformation|GetActorLocation (Variables|Default|GetTargetActor)) (Variables|Default|GetPositionOffset))))
    (:then_1
      (EventDispatchers|BindEventtoMoverEventDispatcher (Actor|GetComponentbyClass (Variables|Default|GetTriggerActor) "/Game/Mover_BP.Mover_BP_C") (delegate Custom|TriggerEvent)))))

(event EventTick
  (params (DeltaSeconds :type Float%20%28single-precision%29))
  (if (Variables|Default|GetAllowMovement)
    (bind _output_get (Variables|Default|SetCurrentPosition (+ (Transformation|GetActorLocation (Variables|Default|GetTargetActor)) (* (Variables|Default|GetDeltaMove) DeltaSeconds))))
    (Math|Float|CompareFloat (Math|Vector|VectorLength (- _output_get (Variables|Default|GetPositionOffset))) 5.0
      (:>
        (Transformation|SetActorLocation (Variables|Default|GetTargetActor) (Variables|Default|GetCurrentPosition) false false))
      (:<
        (EventDispatchers|UnbindEventfromMoverEventDispatcher (Actor|GetComponentbyClass (Variables|Default|GetTriggerActor) "/Game/Mover_BP.Mover_BP_C") (delegate Custom|CustomEvennt))
        (Variables|Default|SetAllowMovement false)))))