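; Spawnable Blueprint that fakes spawning by moving an existing TargetActor above its starting point and revealing it when triggered.
; On BeginPlay it stores the target's location and binds TriggerEvent to the event dispatcher of the Spawner component on TriggerActor.
; When triggered, it teleports the target to that location plus a vertical SpawnOffset, then enables gravity and visibility if it is a StaticMeshActor.
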(event Custom|TriggerEvent
  (Transformation|SetActorLocation (Variables|Default|GetTargetActor) (+ (Variables|Default|GetInitial%20Position) (Math|Vector|MakeVector 0.0 0.0 (Variables|Default|GetSpawnOffset))) false false)
  (bind _asstatic_mesh_actor (Utilities|Casting|CastToStaticMeshActor (Variables|Default|GetTargetActor)))
  (Physics|SetEnableGravity (Variables|/Script/Engine.StaticMeshActor|GetStaticMeshComponent _asstatic_mesh_actor) true)
  (Rendering|SetVisibility (Variables|/Script/Engine.StaticMeshActor|GetStaticMeshComponent _asstatic_mesh_actor) true false))

(event EventBeginPlay
  (Utilities|FlowControl|Sequence
    (:then_0
      (Variables|Default|SetInitial%20Position (Transformation|GetActorLocation (Variables|Default|GetTargetActor))))
    (:then_1
      (EventDispatchers|BindEventtoSpawnerEventDispatcher (Actor|GetComponentbyClass (Variables|Default|GetTriggerActor) "/Game/Spawner.Spawner_C") (delegate Custom|TriggerEvent)))))