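; Trigger actor that teleports the player pawn to the position of a referenced NewPlayerPositionActor.
; It caches that actor's location on BeginPlay, so later movement of the actor is not tracked.
; Any actor overlap moves player pawn 0 there without sweep, regardless of what overlapped, and hides the target actor's root component.
; It then plays the Teleport sound at the trigger's own location.
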(event EventBeginPlay
  (Variables|Default|SetNewPosition (Transformation|GetActorLocation (Variables|Default|GetNewPlayerPositionActor))))

(event Collision|EventActorBeginOverlap
  (params (OtherActor :type Actor%20Object%20Reference))
  (Utilities|FlowControl|Sequence
    (:then_0
      (Transformation|SetActorLocation (Game|Player|GetPlayerPawn 0) (Variables|Default|GetNewPosition) false false)
      (Rendering|SetVisibility (Variables|/Script/Engine.Actor|GetRootComponent (Variables|Default|GetNewPlayerPositionActor)) false false))
    (:then_1
      (Audio|PlaySoundatLocation "/Game/Audio/teleport.teleport" (Transformation|GetActorLocation)))))

(fn ConstructionScript)