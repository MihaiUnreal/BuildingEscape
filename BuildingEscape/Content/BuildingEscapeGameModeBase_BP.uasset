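; Game mode for Building Escape that saves and restores the player pawn's position through a MySaveGame object in a single save slot.
; BeginPlay loads an existing save and moves the pawn there, or creates one from the current position, then prints key instructions.
; Tick polls key 1 to save and key 2 to load, reusing the BeginPlay logic only if the slot exists, with on-screen debug messages.
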(event EventBeginPlay
  (bind _returnvalue (Game|Player|GetPlayerPawn 0))
  (bind _returnvalue_2 (Transformation|GetActorLocation _returnvalue))
  (Utilities|FlowControl|Sequence
    (:then_0
      (bind _returnvalue_3 (SaveGame|DoesSaveGameExist "SaveGame1"))
      (if _returnvalue_3
        (bind _returnvalue_4 (SaveGame|LoadGamefromSlot "SaveGame1"))
        (bind _asmy_save_game (Utilities|Casting|CastToMySaveGame _returnvalue_4)
          (:then
            (bind _output_get (Variables|Default|SetLocalSaveGame _asmy_save_game))
            (bind _returnvalue_5 (Transformation|SetActorLocation (Game|Player|GetPlayerPawn 0) (Variables|/Game/MySaveGame.MySaveGame_C|GetPlayerPosition _output_get) false false))
            (Development|PrintString "Game Loaded" _returnvalue_5 _returnvalue_5 "(R=0.017667,G=0.000000,B=1.000000,A=1.000000)" 3.0)
            (Development|PrintString (Utilities|String|ToString(Vector) (Transformation|GetActorLocation (Game|Player|GetPlayerPawn 0))) true true "(R=0.000000,G=0.047595,B=1.000000,A=1.000000)" 3.0))
          (:CastFailed
            (Development|PrintString "Failed to load game ..." true true "(R=1.000000,G=0.008024,B=0.000000,A=1.000000)" 3.0)))
        (else
          (bind _returnvalue_6 (SaveGame|CreateSaveGameObject "/Game/MySaveGame.MySaveGame_C"))
          (bind _output_get_2 (Variables|Default|SetLocalSaveGame _returnvalue_6))
          (Variables|/Game/MySaveGame.MySaveGame_C|SetPlayerPosition _output_get_2 _returnvalue_2)
          (bind _returnvalue_7 (SaveGame|SaveGametoSlot _output_get_2 "SaveGame1"))
          (Development|PrintString "Game Saved" _returnvalue_7 _returnvalue_7 "(R=0.108544,G=1.000000,B=0.040252,A=1.000000)" 3.0)
          (Development|PrintString (Utilities|String|ToString(Vector) _returnvalue_2) true true "(R=0.000000,G=1.000000,B=0.088856,A=1.000000)" 3.0))))
    (:then_1
      (Development|PrintString "Press 1 to Save Game and 2 to Load Game" true true "(R=1.000000,G=0.438635,B=0.000000,A=1.000000)" 4.0))))

(event EventTick
  (params (DeltaSeconds :type Float%20%28single-precision%29))
  (bind _returnvalue (Game|Player|GetPlayerPawn 0))
  (bind _returnvalue_2 (Game|GetPlayerController 0))
  (bind _returnvalue_3 (Transformation|GetActorLocation _returnvalue))
  (Utilities|FlowControl|Sequence
    (:then_0
      (Variables|Default|SetIsLoadGame (Game|Player|WasInputKeyJustPressed _returnvalue_2 "Two")))
    (:then_1
      (if (Variables|Default|GetIsLoadGame)
        (bind _returnvalue_4 (SaveGame|DoesSaveGameExist "SaveGame1"))
        (if _returnvalue_4
          (bind _returnvalue_5 (SaveGame|LoadGamefromSlot "SaveGame1"))
          (bind _asmy_save_game (Utilities|Casting|CastToMySaveGame _returnvalue_5)
            (:then
              (bind _output_get (Variables|Default|SetLocalSaveGame _asmy_save_game))
              (bind _returnvalue_6 (Transformation|SetActorLocation (Game|Player|GetPlayerPawn 0) (Variables|/Game/MySaveGame.MySaveGame_C|GetPlayerPosition _output_get) false false))
              (Development|PrintString "Game Loaded" _returnvalue_6 _returnvalue_6 "(R=0.017667,G=0.000000,B=1.000000,A=1.000000)" 3.0)
              (Development|PrintString (Utilities|String|ToString(Vector) (Transformation|GetActorLocation (Game|Player|GetPlayerPawn 0))) true true "(R=0.000000,G=0.047595,B=1.000000,A=1.000000)" 3.0))
            (:CastFailed
              (Development|PrintString "Failed to load game ..." true true "(R=1.000000,G=0.008024,B=0.000000,A=1.000000)" 3.0)))
          (else
            (Development|PrintString "Failed to load game ..." true true "(R=1.000000,G=0.049340,B=0.009540,A=1.000000)" 3.0)))))
    (:then_2
      (Variables|Default|SetIsSaveGame (Game|Player|WasInputKeyJustPressed _returnvalue_2 "One")))
    (:then_3
      (if (Variables|Default|GetIsSaveGame)
        (bind _returnvalue_7 (SaveGame|DoesSaveGameExist "SaveGame1"))
        (if _returnvalue_7
          (Variables|/Game/MySaveGame.MySaveGame_C|SetPlayerPosition (stale EventBeginPlay _output_get_2) _returnvalue_3)
          (bind _returnvalue_8 (SaveGame|SaveGametoSlot (stale EventBeginPlay _output_get_2) "SaveGame1"))
          (Development|PrintString "Game Saved" _returnvalue_8 _returnvalue_8 "(R=0.108544,G=1.000000,B=0.040252,A=1.000000)" 3.0)
          (Development|PrintString (Utilities|String|ToString(Vector) _returnvalue_3) true true "(R=0.000000,G=1.000000,B=0.088856,A=1.000000)" 3.0)
          (else
            (Development|PrintString "Failed to save game ..." true true "(R=1.000000,G=0.000000,B=0.000000,A=1.000000)" 3.0)))))))

(fn ConstructionScript)