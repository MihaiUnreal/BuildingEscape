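; HUD Blueprint that shows the main GUI and a temporary on-screen text message.
; On BeginPlay it creates the GUI widget for the owning player and adds it to the viewport.
; DrawHUD draws the Text variable in the given Color at a fixed screen position, then clears it once the TextHideDelay Delay completes.
; Nothing in this graph sets a new message.
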(event EventBeginPlay
  (bind _returnvalue (UserInterface|CreateWidget "/Game/GUI.GUI_C" (Game|Player|GetOwningPlayerController)))
  (UserInterface|Viewport|AddtoViewport _returnvalue 0))

(event EventDrawHUD
  (params (SizeX :type Integer) (SizeY :type Integer))
  (if true
    (HUD|DrawText (Variables|Default|GetText) (Variables|Default|GetColor) 5e+01 5e+01 0 2.0 false)
    (Utilities|FlowControl|Delay (Variables|Default|GetTextHideDelay))
    (Variables|Default|SetText "")))

(fn ConstructionScript)